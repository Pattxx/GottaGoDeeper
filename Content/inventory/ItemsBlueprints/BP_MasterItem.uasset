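; BP_MasterItem is a pickup item actor, apparently the base for inventory items, that the player collects with the E key.
; Overlapping its Collision component with a testinventory actor caches that actor and enables input on the item, while ending the overlap disables it.
; Pressing E passes ItemInfo to the cached actor's PickItem, then destroys the item.
; The end-overlap handler does not check which actor left.
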(event OnComponentBeginOverlap(Collision)
  (params (OverlappedComponent :type Primitive%20Component%20Object%20Reference) (OtherActor :type Actor%20Object%20Reference) (OtherComp :type Primitive%20Component%20Object%20Reference) (OtherBodyIndex :type Integer) (bFromSweep :type Boolean) (SweepResult :type Hit%20Result%20Structure%20%28by%20ref%29))
  ;[0.15 0.15 0.15 0.5] Collision Input
  (bind _astestinventory (Utilities|Casting|CastTotestinventory OtherActor))
  (Variables|Default|SetCharacterCast _astestinventory)
  (Input|EnableInput (Game|GetPlayerController 0)))

(event OnComponentEndOverlap(Collision)
  (params (OverlappedComponent :type Primitive%20Component%20Object%20Reference) (OtherActor :type Actor%20Object%20Reference) (OtherComp :type Primitive%20Component%20Object%20Reference) (OtherBodyIndex :type Integer))
  ;[0.15 0.15 0.15 0.5] Collision Input
  (Input|DisableInput (Game|GetPlayerController 0)))

(event Input|KeyboardEvents|E
  (params (Key :type Key%20Structure :default "None"))
  (:Pressed
    (Default|PickItem (Variables|Default|GetCharacterCast) (Variables|Default|GetItemInfo))
    (Actor|DestroyActor)))

(fn ConstructionScript)