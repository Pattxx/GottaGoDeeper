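; BP_PerunStatue is the puzzle controller for the Perun riddle minigame, checking four face values against a fixed solution.
; On BeginPlay it finds the four BP_ButtonFace actors by class and binds a check event to each.
; Every check calls IsAnswerRight, which on a full match destroys the BP_BlockingFace actor and calls Wygrana (win).
; The face values are only read here, never set.
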(event Custom|Checker4
  (CallFunction|IsAnswerRight))

(event Custom|Checker1
  (CallFunction|IsAnswerRight))

(event Custom|Checker2
  (CallFunction|IsAnswerRight))

(event Custom|Checker3
  (CallFunction|IsAnswerRight))

(event EventBeginPlay
  (bind _returnvalue (Actor|GetActorOfClass "/Game/BluePrints/MiniGames/ZagadkiPerun/BP_ButtonFace1.BP_ButtonFace1_C"))
  (EventDispatchers|BindEventtoCheck1 _returnvalue (delegate Custom|Checker1))
  (bind _returnvalue_2 (Actor|GetActorOfClass "/Game/BluePrints/MiniGames/ZagadkiPerun/BP_ButtonFace2.BP_ButtonFace2_C"))
  (EventDispatchers|BindEventtoCheck2 _returnvalue_2 (delegate Custom|Checker2))
  (bind _returnvalue_3 (Actor|GetActorOfClass "/Game/BluePrints/MiniGames/ZagadkiPerun/BP_ButtonFace3.BP_ButtonFace3_C"))
  (EventDispatchers|BindEventtoCheck3 _returnvalue_3 (delegate Custom|Checker3))
  (bind _returnvalue_4 (Actor|GetActorOfClass "/Game/BluePrints/MiniGames/ZagadkiPerun/BP_ButtonFace4.BP_ButtonFace4_C"))
  (EventDispatchers|BindEventtoCheck4 _returnvalue_4 (delegate Custom|Checker4)))

(event Collision|EventActorBeginOverlap
  (params (OtherActor :type Actor%20Object%20Reference)))

(event EventTick
  (params (DeltaSeconds :type Float%20%28single-precision%29)))

(fn ConstructionScript)

(fn IsAnswerRight
  (if (Math|Boolean|ANDBoolean (== (Variables|Default|GetFace4Val) 3) (== (Variables|Default|GetFace3Val) 1) (== (Variables|Default|GetFace2Val) 2) (== (Variables|Default|GetFace1Val) 0))
    (bind _returnvalue (Actor|GetActorOfClass "/Game/BluePrints/MiniGames/ZagadkiPerun/BP_BlockingFace.BP_BlockingFace_C"))
    (Actor|DestroyActor _returnvalue)
    (Default|CallWygrana)))