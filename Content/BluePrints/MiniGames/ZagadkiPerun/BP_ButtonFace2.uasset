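; Interactable button in the Perun riddle minigame that turns the second face of BP_PerunStatue a quarter turn per press.
; A guard flag blocks presses while a timeline lerps the face's yaw, feeding each result back as the next start value.
; On finish it advances a four-step counter, writes it to the statue's Face2Val and calls Check2.
; It destroys itself when the statue broadcasts Wygrana (win).
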(event Custom|WyrganaEvent
  (Actor|DestroyActor))

(event EventBeginPlay
  (bind _returnvalue (Actor|GetActorOfClass "/Game/BluePrints/MiniGames/ZagadkiPerun/BP_PerunStatue.BP_PerunStatue_C"))
  (EventDispatchers|BindEventtoWygrana _returnvalue (delegate Custom|WyrganaEvent)))

(event EventInteract
  (params (Player :type BP%20First%20Person%20Character%20Object%20Reference))
  (if (not (Variables|Default|GetRot))
    (Variables|Default|SetRot true)
    (bind _returnvalue (Actor|GetActorOfClass "/Game/BluePrints/MiniGames/ZagadkiPerun/BP_PerunStatue.BP_PerunStatue_C"))
    (Variables|Default|SetTargetRotation (+ (Variables|Default|GetCurrentRotation) 9e+01))
    (bind _alpha (Timeline|Timeline PlayFromStart)
      (:Update
        (bind _output_get (Variables|Default|SetCurrentRotation (.z (Math|Vector|Lerp(Vector) (Math|Vector|MakeVector (.roll (Variables|/Script/Engine.SceneComponent|GetRelativeRotation (Variables|/Game/BluePrints/MiniGames/ZagadkiPerun/BP_PerunStatue.BP_PerunStatue_C|GetFace2 _returnvalue))) (.pitch (Variables|/Script/Engine.SceneComponent|GetRelativeRotation (Variables|/Game/BluePrints/MiniGames/ZagadkiPerun/BP_PerunStatue.BP_PerunStatue_C|GetFace2 _returnvalue))) (Variables|Default|GetCurrentRotation)) (Math|Vector|MakeVector (.roll (Variables|/Script/Engine.SceneComponent|GetRelativeRotation (Variables|/Game/BluePrints/MiniGames/ZagadkiPerun/BP_PerunStatue.BP_PerunStatue_C|GetFace2 _returnvalue))) (.pitch (Variables|/Script/Engine.SceneComponent|GetRelativeRotation (Variables|/Game/BluePrints/MiniGames/ZagadkiPerun/BP_PerunStatue.BP_PerunStatue_C|GetFace2 _returnvalue))) (Variables|Default|GetTargetRotation)) _alpha))))
        (Transformation|SetRelativeRotation (Variables|/Game/BluePrints/MiniGames/ZagadkiPerun/BP_PerunStatue.BP_PerunStatue_C|GetFace2 _returnvalue) (Math|Rotator|MakeRotator (.x (Math|Vector|Lerp(Vector) (Math|Vector|MakeVector (.roll (Variables|/Script/Engine.SceneComponent|GetRelativeRotation (Variables|/Game/BluePrints/MiniGames/ZagadkiPerun/BP_PerunStatue.BP_PerunStatue_C|GetFace2 _returnvalue))) (.pitch (Variables|/Script/Engine.SceneComponent|GetRelativeRotation (Variables|/Game/BluePrints/MiniGames/ZagadkiPerun/BP_PerunStatue.BP_PerunStatue_C|GetFace2 _returnvalue))) (Variables|Default|GetCurrentRotation)) (Math|Vector|MakeVector (.roll (Variables|/Script/Engine.SceneComponent|GetRelativeRotation (Variables|/Game/BluePrints/MiniGames/ZagadkiPerun/BP_PerunStatue.BP_PerunStatue_C|GetFace2 _returnvalue))) (.pitch (Variables|/Script/Engine.SceneComponent|GetRelativeRotation (Variables|/Game/BluePrints/MiniGames/ZagadkiPerun/BP_PerunStatue.BP_PerunStatue_C|GetFace2 _returnvalue))) (Variables|Default|GetTargetRotation)) _alpha)) (.y (Math|Vector|Lerp(Vector) (Math|Vector|MakeVector (.roll (Variables|/Script/Engine.SceneComponent|GetRelativeRotation (Variables|/Game/BluePrints/MiniGames/ZagadkiPerun/BP_PerunStatue.BP_PerunStatue_C|GetFace2 _returnvalue))) (.pitch (Variables|/Script/Engine.SceneComponent|GetRelativeRotation (Variables|/Game/BluePrints/MiniGames/ZagadkiPerun/BP_PerunStatue.BP_PerunStatue_C|GetFace2 _returnvalue))) (Variables|Default|GetCurrentRotation)) (Math|Vector|MakeVector (.roll (Variables|/Script/Engine.SceneComponent|GetRelativeRotation (Variables|/Game/BluePrints/MiniGames/ZagadkiPerun/BP_PerunStatue.BP_PerunStatue_C|GetFace2 _returnvalue))) (.pitch (Variables|/Script/Engine.SceneComponent|GetRelativeRotation (Variables|/Game/BluePrints/MiniGames/ZagadkiPerun/BP_PerunStatue.BP_PerunStatue_C|GetFace2 _returnvalue))) (Variables|Default|GetTargetRotation)) _alpha)) _output_get) false false))
      (:Finished
        (Variables|Default|SetCurrentRotation (Variables|Default|GetTargetRotation))
        (Variables|Default|SetCurrentRotation (Math|Float|%(Float) (Variables|Default|GetCurrentRotation) 3.6e+02))
        (Variables|Default|SetTargetRotation (Math|Float|%(Float) (Variables|Default|GetTargetRotation) 3.6e+02))
        (Variables|Default|SetDoVal (Math|Integer|%(Integer) (+ (Variables|Default|GetDoVal) 1) 4))
        (Variables|/Game/BluePrints/MiniGames/ZagadkiPerun/BP_PerunStatue.BP_PerunStatue_C|SetFace2Val _returnvalue (Variables|Default|GetDoVal))
        (Variables|Default|SetRot false)
        (Default|CallCheck2)))))

(fn ConstructionScript
  (|CallParentFunction))