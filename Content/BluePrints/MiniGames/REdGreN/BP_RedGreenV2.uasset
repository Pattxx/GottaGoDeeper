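; Red Light, Green Light minigame actor, started on the server by BP_BabaJagaStart's event.
; A delay in Tick flips the phase every 3–4 seconds, turning the head with timelines and stopping or respawning the music.
; While red, a looping timer teleports player 0 to a fixed point if moving; a similar Player2 check exists, but Player2 is never assigned.
; Any Sphere overlap toggles the music and destroys the actor.
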(event OnComponentBeginOverlap(Sphere)
  (params (OverlappedComponent :type Primitive%20Component%20Object%20Reference) (OtherActor :type Actor%20Object%20Reference) (OtherComp :type Primitive%20Component%20Object%20Reference) (OtherBodyIndex :type Integer) (bFromSweep :type Boolean) (SweepResult :type Hit%20Result%20Structure%20%28by%20ref%29))
  (Components|Activation|ToggleActive (Variables|Default|GetSound))
  (Actor|DestroyActor))

(event Custom|Start
  (Networking|SwitchHasAuthority
    (:Authority
      (bind _asbp_first_person_character (Utilities|Casting|CastToBP_FirstPersonCharacter (Game|GetPlayerCharacter 0)))
      (Variables|Default|SetPlayer _asbp_first_person_character)
      (Variables|Default|SetGameStarted true)
      (Utilities|Time|SetTimerbyEvent (delegate Custom|IsPlayerMoving) 0.1 true)
      (Utilities|Time|SetTimerbyEvent 0 0.0)
      (bind _returnvalue (Audio|SpawnSound2D "/Game/CavesAndDungeons/CUE/CUE_Ethereal_Rites_Loop_A_Cue.CUE_Ethereal_Rites_Loop_A_Cue" 1.0 1.0 0.0 0))
      (Variables|Default|SetSound _returnvalue))))

(event Custom|SecondPlayerMoving
  (if (and (Variables|Default|GetisRed) (>= (Math|Vector|VectorLength (Variables|/Script/Engine.MovementComponent|GetVelocity (Variables|/Script/Engine.Character|GetCharacterMovement (Variables|Default|GetPlayer2)))) 3.0))
    (Transformation|SetActorLocation (Variables|Default|GetPlayer2) "9650.000000,-4770.000000,2220.000000" false false)))

(event Custom|HeadRotation
  (bind __head (Variables|Default|Get%20Head))
  (bind __head_2 (Variables|Default|Get%20Head))
  (bind _relativerotation (Variables|/Script/Engine.SceneComponent|GetRelativeRotation __head))
  (bind _relativerotation_2 (Variables|/Script/Engine.SceneComponent|GetRelativeRotation __head_2))
  (Utilities|FlowControl|FlipFlop
    (:A
      (Components|Activation|ToggleActive (Variables|Default|GetSound))
      (bind _alpha (Timeline|Timeline PlayFromStart)
        (:Update
          (Transformation|SetRelativeRotation (Variables|Default|Get%20Head) (Math|Rotator|MakeRotator (.x (Math|Vector|Lerp(Vector) (Math|Vector|MakeVector (.roll _relativerotation_2) (.pitch _relativerotation_2) (.yaw _relativerotation_2)) "0, 0, 0" _alpha)) (.y (Math|Vector|Lerp(Vector) (Math|Vector|MakeVector (.roll _relativerotation_2) (.pitch _relativerotation_2) (.yaw _relativerotation_2)) "0, 0, 0" _alpha)) (.z (Math|Vector|Lerp(Vector) (Math|Vector|MakeVector (.roll _relativerotation_2) (.pitch _relativerotation_2) (.yaw _relativerotation_2)) "0, 0, 0" _alpha))) false false))
        (:Finished
          (Variables|Default|SetisRed true))))
    (:B
      (Variables|Default|SetisRed false)
      (bind _returnvalue (Audio|SpawnSound2D "/Game/CavesAndDungeons/CUE/CUE_Ethereal_Rites_Loop_A_Cue.CUE_Ethereal_Rites_Loop_A_Cue" 1.0 1.0 0.0 0))
      (Variables|Default|SetSound _returnvalue)
      (bind _alpha_2 (Timeline|Timeline_0 PlayFromStart)
        (:Update
          (Transformation|SetRelativeRotation (Variables|Default|Get%20Head) (Math|Rotator|MakeRotator (.x (Math|Vector|Lerp(Vector) (Math|Vector|MakeVector (.roll _relativerotation) (.pitch _relativerotation) (.yaw _relativerotation)) "0.000000,0.000000,180.000000" _alpha_2)) (.y (Math|Vector|Lerp(Vector) (Math|Vector|MakeVector (.roll _relativerotation) (.pitch _relativerotation) (.yaw _relativerotation)) "0.000000,0.000000,180.000000" _alpha_2)) (.z (Math|Vector|Lerp(Vector) (Math|Vector|MakeVector (.roll _relativerotation) (.pitch _relativerotation) (.yaw _relativerotation)) "0.000000,0.000000,180.000000" _alpha_2))) false false))))))

(event Custom|IsPlayerMoving
  (if (and (Variables|Default|GetisRed) (>= (Math|Vector|VectorLength (Variables|/Script/Engine.MovementComponent|GetVelocity (Variables|/Script/Engine.Character|GetCharacterMovement (Variables|Default|GetPlayer)))) 3.0))
    (Transformation|SetActorLocation (Variables|Default|GetPlayer) "9650.000000,-4770.000000,2220.000000" false false)))

(event EventBeginPlay
  (bind _returnvalue (Actor|GetActorOfClass "/Game/BluePrints/MiniGames/REdGreN/BP_BabaJagaStart.BP_BabaJagaStart_C"))
  (EventDispatchers|BindEventtoStartBaba _returnvalue (delegate Custom|Start)))

(event EventTick
  (params (DeltaSeconds :type Float%20%28single-precision%29))
  (if (Variables|Default|GetGameStarted)
    (Utilities|FlowControl|Delay (Math|Random|RandomFloatinRange 3.0 4.0))
    (CallFunction|HeadRotation)))

(fn ConstructionScript)