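; Start trigger actor for the Baba Jaga (red light, green light) minigame that notifies a target as players enter its collision.
; It caches BP_GDD_GameMode shortly after BeginPlay and compares overlapping actors against Gracz1, treating any other actor as Gracz2.
; Each branch sends CharacterTriggerMessage with that player to Target once via DoOnce and increments a counter.
; The actor destroys itself when the counter reaches two.
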(event OnComponentBeginOverlap(Colision)
  (params (OverlappedComponent :type Primitive%20Component%20Object%20Reference) (OtherActor :type Actor%20Object%20Reference) (OtherComp :type Primitive%20Component%20Object%20Reference) (OtherBodyIndex :type Integer) (bFromSweep :type Boolean) (SweepResult :type Hit%20Result%20Structure%20%28by%20ref%29))
  (bind _target (Variables|Default|GetTarget))
  (bind _gamemode (Variables|Default|GetGameMode))
  (bind _gracz1 (Variables|/Game/BluePrints/BP_GDD_GameMode.BP_GDD_GameMode_C|GetGracz1 _gamemode))
  (if (== OtherActor _gracz1)
    (Utilities|FlowControl|DoOnce false
      (:Completed
        (Class|BPIBabaJaga|CharacterTrigger(Message) _target _gracz1)
        (Math|Integer|IncrementInt (Variables|Default|GetCount)
          (:%20%20
            _))))
    (else
      (Utilities|FlowControl|DoOnce false
        (:Completed
          (Class|BPIBabaJaga|CharacterTrigger(Message) _target (Variables|/Game/BluePrints/BP_GDD_GameMode.BP_GDD_GameMode_C|GetGracz2 (Variables|Default|GetGameMode)))
          (Math|Integer|IncrementInt (Variables|Default|GetCount)
            (:%20%20
              _))))))
  (if (== (Variables|Default|GetCount) 2)
    (Actor|DestroyActor)))

(event EventBeginPlay
  (Utilities|FlowControl|Delay 0.2)
  (bind _asbp_gdd_game_mode (Utilities|Casting|CastToBP_GDD_GameMode (Game|GetGameMode))
    (:then
      (Variables|Default|SetGameMode _asbp_gdd_game_mode))
    (:CastFailed
      (Development|PrintString "Hello"))))

(event Collision|EventActorBeginOverlap
  (params (OtherActor :type Actor%20Object%20Reference)))

(event EventTick
  (params (DeltaSeconds :type Float%20%28single-precision%29)))

(fn ConstructionScript)