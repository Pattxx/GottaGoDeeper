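; Base pickup item for the interaction system, with a widget that appears when the first-person character enters its sphere.
; End overlap hides the widget for any actor, without a character check.
; On Interact, it passes the held item class, its own class and item details to the player's PickupItem, then has the player destroy it through DestroyPickItem.
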(event OnComponentBeginOverlap(Sphere)
  (params (OverlappedComponent :type Primitive%20Component%20Object%20Reference) (OtherActor :type Actor%20Object%20Reference) (OtherComp :type Primitive%20Component%20Object%20Reference) (OtherBodyIndex :type Integer) (bFromSweep :type Boolean) (SweepResult :type Hit%20Result%20Structure%20%28by%20ref%29))
  (if (!= OtherActor self)
    (Utilities|Casting|CastToBP_FirstPersonCharacter OtherActor)
    (Rendering|SetVisibility (Variables|Default|GetWidget) true false)))

(event OnComponentEndOverlap(Sphere)
  (params (OverlappedComponent :type Primitive%20Component%20Object%20Reference) (OtherActor :type Actor%20Object%20Reference) (OtherComp :type Primitive%20Component%20Object%20Reference) (OtherBodyIndex :type Integer))
  (Rendering|SetVisibility (Variables|Default|GetWidget) false false))

(event EventInteract
  (params (Player :type BP%20First%20Person%20Character%20Object%20Reference))
  (bind _self self)
  (Default|PickupItem Player (Variables|Default|GetCurrentlyHeldItem) (Utilities|GetClass _self) (Variables|Default|GetitemDet))
  (Default|DestroyPickItem Player _self))

(fn ConstructionScript)