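; BP_CaveGenerator is an unfinished procedural cave generator actor that begins generation on the server shortly after BeginPlay.
; GenerateCave currently only looks up a BP_StartCave actor and prints whether one was found.
; Disconnected nodes sketch storing that reference, spawning a random CaveTypes piece at an exit transform, and repositioning it, but none of them execute.
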(event EventBeginPlay
  (Networking|SwitchHasAuthority
    (:Authority
      (Utilities|FlowControl|Delay 0.2)
      (CallFunction|GenerateCave))))

(event Collision|EventActorBeginOverlap
  (params (OtherActor :type Actor%20Object%20Reference)))

(event EventTick
  (params (DeltaSeconds :type Float%20%28single-precision%29)))

(fn ConstructionScript)

(fn GenerateCave
  (bind _returnvalue (Actor|GetActorOfClass "/Game/BluePrints/CaveGen/BP_StartCave.BP_StartCave_C"))
  (Utilities|IsValid _returnvalue
    (:Is%20Valid
      (Development|PrintString "Ok"))
    (:Is%20Not%20Valid
      (Development|PrintString "No Start Cave"))))