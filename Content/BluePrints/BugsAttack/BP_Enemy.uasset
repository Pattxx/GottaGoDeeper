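; BP_Enemy is an enemy character in BugsAttack that slowly chases the player.
; From BeginPlay it runs a repeating AI MoveTo toward the player, pausing a second after each finished move.
; Its Sphere overlap calls DecreaseHunger on BP_FirstPersonCharacter once per entry, passing a negative amount.
; When the player leaves the sphere, it clears an Attack flag, which is never set or read here.
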(event OnComponentBeginOverlap(Sphere)
  (params (OverlappedComponent :type Primitive%20Component%20Object%20Reference) (OtherActor :type Actor%20Object%20Reference) (OtherComp :type Primitive%20Component%20Object%20Reference) (OtherBodyIndex :type Integer) (bFromSweep :type Boolean) (SweepResult :type Hit%20Result%20Structure%20%28by%20ref%29))
  (bind _asrandom (Utilities|Casting|CastToBP_FirstPersonCharacter OtherActor))
  (Default|DecreaseHunger _asrandom -1.0))

(event OnComponentEndOverlap(Sphere)
  (params (OverlappedComponent :type Primitive%20Component%20Object%20Reference) (OtherActor :type Actor%20Object%20Reference) (OtherComp :type Primitive%20Component%20Object%20Reference) (OtherBodyIndex :type Integer))
  (if (== OtherActor (Game|GetPlayerCharacter 0))
    (Variables|Default|SetAttack false)))

(event EventBeginPlay
  (Variables|/Script/Engine.CharacterMovementComponent|SetMaxWalkSpeed (Variables|Character|GetCharacterMovement) 1e+02)
  (AI|AIMoveTo (AI|GetAIController self) "0, 0, 0" (Game|GetPlayerCharacter 0) -1.0 "Default" "Default" true true :!label _label
    (:OnMoveFinished
      (Utilities|FlowControl|Delay 1.0)
      (goto _label))))

(fn ConstructionScript)