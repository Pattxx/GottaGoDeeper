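; BP_Spawner is a triggered enemy spawner for a timed BugsAttack wave, activated when the first-person character enters its sphere.
; After an initial delay, a looping timer spawns BP_Enemy slightly raised at random angles on the sphere's radius while CanSpawn is true.
; A minute after overlap it destroys itself and all enemies, then spawns two BP_Mozd1 actors at hardcoded transforms.
; The construction script sizes the sphere from Radius.
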(event OnComponentBeginOverlap(Sphere)
  (params (OverlappedComponent :type Primitive%20Component%20Object%20Reference) (OtherActor :type Actor%20Object%20Reference) (OtherComp :type Primitive%20Component%20Object%20Reference) (OtherBodyIndex :type Integer) (bFromSweep :type Boolean) (SweepResult :type Hit%20Result%20Structure%20%28by%20ref%29))
  (Utilities|Casting|CastToBP_FirstPersonCharacter OtherActor)
  (Utilities|Time|SetTimerbyEvent (delegate Custom|spawningEvent) 0.5 true false 5.0)
  (Utilities|FlowControl|Delay 6e+01)
  (Actor|DestroyActor)
  (bind _outactors (Actor|GetAllActorsOfClass "/Game/BluePrints/BugsAttack/BP_Enemy.BP_Enemy_C"))
  (for _array_element _outactors
    (Actor|DestroyActor _array_element))
  (Game|SpawnActorfromClass "/Game/BluePrints/BugsAttack/BP_Mozd1.BP_Mozd1_C" (Math|Transform|MakeTransform "19340.000000,-16350.000000,3320.000000" "10.000000,0.000000,0.000000" "1.000000,1.000000,1.000000") "Undefined" "MultiplyWithRoot" 0 0)
  (Game|SpawnActorfromClass "/Game/BluePrints/BugsAttack/BP_Mozd1.BP_Mozd1_C" (Math|Transform|MakeTransform "17030.000000,-18540.000000,2940.000000" "-20.000000,0.000000,0.000000" "1.000000,1.000000,1.000000") "Undefined" "MultiplyWithRoot" 0 0))

(event Custom|spawningEvent
  (bind _returnvalue (Math|Random|RandomFloatinRange 0.0 3.6e+02))
  (bind _returnvalue_2 (Transformation|GetActorLocation))
  (bind _radius (Variables|Default|GetRadius))
  (bind _returnvalue_3 (Math|Vector|RotateVector (Math|Vector|MakeVector _radius 0.0 0.0) (Math|Rotator|MakeRotator 0.0 0.0 _returnvalue)))
  (bind _returnvalue_4 (+ _returnvalue_3 _returnvalue_2))
  (bind (_x _y _z) (Math|Vector|BreakVector _returnvalue_4))
  (if (Variables|Default|GetCanSpawn)
    (Game|SpawnActorfromClass "/Game/BluePrints/BugsAttack/BP_Enemy.BP_Enemy_C" (Math|Transform|MakeTransform (Math|Vector|MakeVector _x _y (+ _z 1e+02)) "0, 0, 0" "1.000000,1.000000,1.000000") "Undefined" "MultiplyWithRoot" 0 0)))

(fn ConstructionScript
  (Components|Sphere|SetSphereRadius (Variables|Default|GetSphere) (Variables|Default|GetRadius) true))