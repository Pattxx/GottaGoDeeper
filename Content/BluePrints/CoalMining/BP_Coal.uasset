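; BP_Coal is an interactable coal deposit that runs a mining minigame and yields mined coal.
; Interact toggles the player's CoalMiningWidget, mining state, mouse cursor and input mode, and binds to the widget's BarFull event.
; When the bar fills, it spawns BP_CoalMined beside itself, closes the minigame and increments a use counter (IleUzyc), destroying itself after three uses.
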(event Custom|MinigameDone
  (bind _returnvalue (Game|GetPlayerController 0))
  (Game|SpawnActorfromClass "/Game/BluePrints/CoalMining/BP_CoalMined.BP_CoalMined_C" (Math|Transform|MakeTransform (+ (Transformation|GetActorLocation) "0.000000,20.000000,0.000000") "0, 0, 0" "1.000000,1.000000,1.000000") "Undefined" "MultiplyWithRoot" 0 0)
  (Input|SetInputModeGameOnly _returnvalue false)
  (Widget|SetVisibility (Variables|Default|GetCoalWidget) "Hidden")
  (Variables|/Game/FirstPerson/Blueprints/BP_FirstPersonCharacter.BP_FirstPersonCharacter_C|SetIsMining? (Variables|Default|GetPlayer) false)
  (Variables|/Script/Engine.PlayerController|SetbShowMouseCursor _returnvalue false)
  (Variables|Default|SetWillShow true)
  (Math|Integer|IncrementInt (Variables|Default|GetIleUzyc)
    (:%20%20
      (if (== (Variables|Default|GetIleUzyc) 3)
        (Actor|DestroyActor)))))

(event EventBeginPlay)

(event Collision|EventActorBeginOverlap
  (params (OtherActor :type Actor%20Object%20Reference)))

(event EventTick
  (params (DeltaSeconds :type Float%20%28single-precision%29)))

(event EventInteract
  (params (Player :type BP%20First%20Person%20Character%20Object%20Reference))
  (bind _returnvalue (Game|GetPlayerController 0))
  (Variables|Default|SetPlayer Player)
  (bind _output_get (Variables|Default|SetCoalWidget (Variables|/Game/FirstPerson/Blueprints/BP_FirstPersonCharacter.BP_FirstPersonCharacter_C|GetCoalMiningWidget Player)))
  (EventDispatchers|BindEventtoBarFull _output_get (delegate Custom|MinigameDone))
  (if (Variables|Default|GetWillShow)
    (Widget|SetVisibility (Variables|Default|GetCoalWidget) "Visible")
    (Variables|/Game/FirstPerson/Blueprints/BP_FirstPersonCharacter.BP_FirstPersonCharacter_C|SetIsMining? (Variables|Default|GetPlayer) true)
    (Variables|/Script/Engine.PlayerController|SetbShowMouseCursor _returnvalue true)
    (Input|SetInputModeGameandUI _returnvalue 0 "DoNotLock" true false)
    (Variables|Default|SetWillShow false)
    (else
      (Widget|SetVisibility (Variables|Default|GetCoalWidget) "Hidden")
      (Variables|/Game/FirstPerson/Blueprints/BP_FirstPersonCharacter.BP_FirstPersonCharacter_C|SetIsMining? (Variables|Default|GetPlayer) false)
      (Variables|/Script/Engine.PlayerController|SetbShowMouseCursor _returnvalue false)
      (Input|SetInputModeGameOnly _returnvalue false)
      (Variables|Default|SetWillShow true))))

(fn ConstructionScript
  (|CallParentFunction))