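; BP_notatnik is an interactable notebook in the CoalMining folder that shows and hides the player's NotkaDucha ("ghost note") widget.
; Its Interact event takes the NotkaDucha widget from the interacting player, then a FlipFlop alternates that widget between Visible and Hidden.
; Each toggle also sets the player's IsReadingNotkaDucha flag to match.
; The toggle state lives in the notebook's FlipFlop, and the player's flag is never read.
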(event EventBeginPlay)

(event Collision|EventActorBeginOverlap
  (params (OtherActor :type Actor%20Object%20Reference)))

(event EventTick
  (params (DeltaSeconds :type Float%20%28single-precision%29)))

(event EventInteract
  (params (Player :type BP%20First%20Person%20Character%20Object%20Reference))
  (Variables|Default|SetPlayer Player)
  (Variables|Default|SetWidgetNotatka (Variables|/Game/FirstPerson/Blueprints/BP_FirstPersonCharacter.BP_FirstPersonCharacter_C|GetNotkaDucha Player))
  (Utilities|FlowControl|FlipFlop
    (:A
      (Widget|SetVisibility (Variables|Default|GetWidgetNotatka) "Visible")
      (Variables|/Game/FirstPerson/Blueprints/BP_FirstPersonCharacter.BP_FirstPersonCharacter_C|SetIsReadingNotkaDucha? (Variables|Default|GetPlayer) true))
    (:B
      (Widget|SetVisibility (Variables|Default|GetWidgetNotatka) "Hidden")
      (Variables|/Game/FirstPerson/Blueprints/BP_FirstPersonCharacter.BP_FirstPersonCharacter_C|SetIsReadingNotkaDucha? (Variables|Default|GetPlayer) false))))

(fn ConstructionScript
  (|CallParentFunction))