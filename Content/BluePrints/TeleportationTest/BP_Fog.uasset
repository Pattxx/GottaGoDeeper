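; BP_Fog is a fog volume actor that tells the first-person character when it is inside the fog.
; On box overlap begin, it passes the character a reference to itself and a fog radius taken from the larger scaled X or Y box extent.
; Overlap begin and end toggle the character's in-fog flag, while the fog's own flag changes for any overlapping actor, before the cast.
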(event OnComponentBeginOverlap(BoxCollision)
  (params (OverlappedComponent :type Primitive%20Component%20Object%20Reference) (OtherActor :type Actor%20Object%20Reference) (OtherComp :type Primitive%20Component%20Object%20Reference) (OtherBodyIndex :type Integer) (bFromSweep :type Boolean) (SweepResult :type Hit%20Result%20Structure%20%28by%20ref%29))
  (bind _boxcollision (Variables|Default|GetBoxCollision))
  (bind _returnvalue (Components|Box|GetScaledBoxExtent _boxcollision))
  (bind (_x _y) (Math|Vector|BreakVector _returnvalue))
  (Variables|Default|SetPlayerIn true)
  (bind _asbp_first_person_character (Utilities|Casting|CastToBP_FirstPersonCharacter OtherActor))
  (Variables|/Game/FirstPerson/Blueprints/BP_FirstPersonCharacter.BP_FirstPersonCharacter_C|SetPlayerIN _asbp_first_person_character true)
  (Variables|/Game/FirstPerson/Blueprints/BP_FirstPersonCharacter.BP_FirstPersonCharacter_C|SetFogRef _asbp_first_person_character self)
  (Variables|/Game/FirstPerson/Blueprints/BP_FirstPersonCharacter.BP_FirstPersonCharacter_C|SetFogRadius _asbp_first_person_character (Math|Float|Max(Float) _x _y)))

(event OnComponentEndOverlap(BoxCollision)
  (params (OverlappedComponent :type Primitive%20Component%20Object%20Reference) (OtherActor :type Actor%20Object%20Reference) (OtherComp :type Primitive%20Component%20Object%20Reference) (OtherBodyIndex :type Integer))
  (Variables|Default|SetPlayerIn false)
  (bind _asbp_first_person_character (Utilities|Casting|CastToBP_FirstPersonCharacter OtherActor))
  (Variables|/Game/FirstPerson/Blueprints/BP_FirstPersonCharacter.BP_FirstPersonCharacter_C|SetPlayerIN _asbp_first_person_character false))

(fn ConstructionScript)